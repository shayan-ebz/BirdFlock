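; BP_FlockManager spawns skeletal-mesh flock components around itself and animates them as a boids-style flock.
; Tick moves each member along its local Y axis while easing rotation toward its DestinationRotation.
; A looping timer alternates between Cohesion, which aims members at the manager, and neighbor gathering plus Separation, which adjusts Destination.
; Alignment, which would convert Destination into rotation, is never called, so only Cohesion steers.
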(event Custom|Update%20Flock%20Behavior
  ;[1 1 1] Updates the status of The Destination And The Rotation of the Flocks by performing 3 main actions on the flocks
  (for (_array_element _array_index) (Variables|Default|GetFlocks)
    (if (Variables|Default|GetbCohesion)
      (CallFunction|Cohesion _array_element)
      (Utilities|FlowControl|Delay (Variables|2)FlockBehavior|GetCohesion%20Delay))
      (Variables|Default|SetbCohesion false)
      (else
        (CallFunction|SetFlockmates _array_element _array_index)
        (CallFunction|Separation _array_element)
        (Utilities|FlowControl|Delay (Variables|2)FlockBehavior|GetCohesion%20Delay))
        (Variables|Default|SetbCohesion true)))))

(event EventBeginPlay
  (bind _returnvalue (Transformation|GetActorLocation))
  ;[1 1 1] Adding Flocks as Skeletal Mesh Component to this Actor
  (for _index (range 0 (- (Variables|1)FlockSpawnEssentials|GetNum%20Flocks) 1))
    (bind _new_location_with_offset (CallFunction|GetRandomOffsetinRangefrom (Variables|1)FlockSpawnEssentials|GetSpawn%20Raduis) _returnvalue))
    (bind _returnvalue_2 (AddComponent|AddBPFlock false (Math|Transform|MakeTransform (- _new_location_with_offset _returnvalue) "0, 0, 0" (Variables|1)FlockSpawnEssentials|GetFlock%20Scale))))
    (Class|SkinnedMeshComponent|SetSkeletalMesh _returnvalue_2 (Variables|1)FlockSpawnEssentials|GetFlock%20Mesh) true)
    (Class|SkeletalMeshComponent|SetAnimClass _returnvalue_2 (Variables|1)FlockSpawnEssentials|GetFlock%20Anim%20Class))
    (Utilities|Array|Add (Variables|Default|GetFlocks) _returnvalue_2)
    ;[1 1 1] Setting Initial Destination for each flock
    (bind _new_location_with_offset_2 (CallFunction|GetRandomOffsetinRangefrom (Variables|1)FlockSpawnEssentials|GetSpawn%20Raduis) (Transformation|GetActorLocation)))
    (Variables|/Game/Flock/BP_Flock.BP_Flock_C|SetDestination _returnvalue_2 _new_location_with_offset_2))
  ;;[1 0.9322 0] End of the Spawning
  (Utilities|Time|SetTimerbyFunctionName self "Update Flock Behavior" (Variables|2)FlockBehavior|GetBehavior%20Update%20Interval) true))

(event EventTick
  (params (DeltaSeconds :type Float%20%28single-precision%29))
  (for _array_element (Variables|Default|GetFlocks)
    (Utilities|FlowControl|Sequence
      (:then_0
        ;[1 1 1] Moving Flocks Forward
        (Transformation|AddLocalOffset _array_element (Math|Vector|MakeVector 0.0 (* (Utilities|Time|GetWorldDeltaSeconds) (Variables|2)FlockBehavior|GetFlock%20Speed)) 0.0) false false))
      (:then_1
        ;[1 1 1] Set the Rotation of the flocks(very important cuz the movement is only in their forward direction)
        (Transformation|SetWorldRotation _array_element (Math|Interpolation|RInterpTo (Transformation|GetWorldRotation _array_element) (Variables|/Game/Flock/BP_Flock.BP_Flock_C|GetDestinationRotation _array_element) (Utilities|Time|GetWorldDeltaSeconds) 1.0) false false)))))

(fn ConstructionScript
  ;[1 1 1] To See the Updates in Editor and Viewport I set the radius in constructor
  (Components|Sphere|SetSphereRadius (Variables|Default|GetSpawn%20Area) (Variables|1)FlockSpawnEssentials|GetSpawn%20Raduis) true))

(fn GetRandomOffsetinRangefrom
  (params (Range :type Float%20%28single-precision%29) (Offset%20Origin :type Vector))
  (bind _returnvalue (* Range -1.0))
  (return (+ (Math|Vector|MakeVector (Math|Random|RandomFloatinRange _returnvalue Range) (Math|Random|RandomFloatinRange _returnvalue Range) (Math|Random|RandomFloatinRange _returnvalue Range)) Offset%20Origin)))

(fn Cohesion
  (params (Flock :type BP%20Flock%20Object%20Reference))
  (bind _returnvalue (Transformation|GetWorldLocation Flock))
  (bind _returnvalue_2 (Transformation|GetActorLocation))
  (bind _returnvalue_3 (- _returnvalue_2 _returnvalue))
  (bind _returnvalue_4 (Math|Conversions|RotationFromXVector _returnvalue_3))
  (Variables|/Game/Flock/BP_Flock.BP_Flock_C|SetDestinationRotation Flock (Math|Rotator|MakeRotator (.roll _returnvalue_4) (.pitch _returnvalue_4) (- (.yaw _returnvalue_4) 9e+01))))

(fn Separation
  (params (Flock :type BP%20Flock%20Object%20Reference))
  (bind _sphereradius (Collision|GetComponentBounds Flock))
  (bind _returnvalue (* _sphereradius 256.0))
  (for (_array_element _array_index) (Variables|/Game/Flock/BP_Flock.BP_Flock_C|GetFlockmates Flock)
    ;[1 1 1] Set The Average Destination of the Flockmates
    (LocalVariables|SetFlockmates%20Destination%20Avg (/ (+ (LocalVariables|GetFlockmates%20Destination%20Avg) (Variables|/Game/Flock/BP_Flock.BP_Flock_C|GetDestination _array_element)) _array_index))
    ;[1 1 1] If a Flockmate is very close to the current flock
    (if (<= (Math|Vector|VectorLength (- (Transformation|GetWorldLocation _array_element) (Transformation|GetWorldLocation Flock))) _sphereradius)
      ;[1 1 1] Then Add the Average Distance of the flockmates + some Randomness to this Flocks Destination
      (Variables|/Game/Flock/BP_Flock.BP_Flock_C|SetDestination Flock (+ (- (LocalVariables|GetFlockmates%20Destination%20Avg) (Transformation|GetWorldLocation Flock)) (Math|Random|RandomFloatinRange (* _returnvalue -1.0) _returnvalue))))))

(fn SetFlockmates
  (params (Flock :type BP%20Flock%20Object%20Reference) (Index :type Integer))
  ;[1 1 1] Clear Current mates to store new ones
  (Utilities|Array|Clear (Variables|/Game/Flock/BP_Flock.BP_Flock_C|GetFlockmates Flock))
  ;[1 1 1] Iterate through all the flocks(except for the current flock) and check to see if there is any flock near than the Flockmate Radius. if it's closer then add to Flockmates of the current flock
  (for (_array_element _array_index) (Variables|Default|GetFlocks)
    (if (!= _array_index Index)
      (if (<= (Math|Vector|VectorLength (- (Transformation|GetWorldLocation _array_element) (Transformation|GetWorldLocation Flock))) (Variables|2)FlockBehavior|GetFlockmate%20Radius))
        (Utilities|Array|Add (Variables|/Game/Flock/BP_Flock.BP_Flock_C|GetFlockmates Flock) _array_element)))))

(fn Alignment
  (params (Flock :type BP%20Flock%20Object%20Reference))
  ;[1 0 0] TODO: since the actor's forward is Y,  I should test this out to see the values
  (Variables|/Game/Flock/BP_Flock.BP_Flock_C|SetDestinationRotation Flock (Math|Conversions|RotationFromXVector (Variables|/Game/Flock/BP_Flock.BP_Flock_C|GetDestination Flock))))